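; BP_Keypad is an interactable code keypad that blends the player's view to its own camera for clickable entry.
; Interact enters keypad view with cursor, click and hover events, or blends back out when OnKeypad is set.
; Setup, also callable through Initiate, masks the display with one dot per KeypadCode character.
; It hands each child-actor button (digits, OK, NO) a reference to the keypad.
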(event Custom|Initiate
  (bind _returnvalue (Game|GetPlayerController 0))
  (bind _code (Variables|Default|GetCode))
  (bind _output_get (Variables|/Script/Engine.PlayerController|SetbShowMouseCursor _returnvalue true))
  (bind _output_get_2 (Variables|/Script/Engine.PlayerController|SetbEnableClickEvents _returnvalue _output_get))
  (Variables|/Script/Engine.PlayerController|SetbEnableMouseOverEvents _returnvalue _output_get_2)
  (Rendering|Components|TextRender|SetText _code (Utilities|Text|MakeLiteralText (Utilities|Text|ToText(String) (Utilities|String|GetSubstring (Utilities|String|MakeLiteralString ".........") 0 (Utilities|String|Len (Variables|Components|GetKeypadCode))))))
  (Rendering|Components|TextRender|SetTextRenderColor _code (Math|Color|MakeColor 20 20 20 255))
  (bind _output_get_3 (Variables|Components|SetButtonsArray (Utilities|Array|MakeArray (Variables|Default|GetButtonNB0) (Variables|Default|GetButtonNB1) (Variables|Default|GetButtonNB2) (Variables|Default|GetButtonNB3) (Variables|Default|GetButtonNB4) (Variables|Default|GetButtonNB5) (Variables|Default|GetButtonNB6) (Variables|Default|GetButtonNB7) (Variables|Default|GetButtonNB8) (Variables|Default|GetButtonNB9) (Variables|Default|GetButtonOK) (Variables|Default|GetButtonNO))))
  (for _array_element _output_get_3
    (bind _asbutton_nb (Utilities|Casting|CastToButtonNB (Variables|/Script/Engine.ChildActorComponent|GetChildActor _array_element)))
    (Variables|/Game/AddedAssets/ButtonNB.ButtonNB_C|SetKeypadActorRef _asbutton_nb self)))

(event EventBeginPlay
  (|CallParentFunction) ; This node is disabled and will not be called.\nDrag off pins to build functionality.
)

(event Collision|EventActorBeginOverlap
  (params (OtherActor :type Actor%20Object%20Reference)))

(event EventTick
  (params (DeltaSeconds :type Float%20%28single-precision%29)))

(event EventInteract
  (bind _returnvalue (Game|GetPlayerController 0))
  (bind _returnvalue_2 (Game|GetPlayerController 0))
  (bind _code (Variables|Default|GetCode))
  (|CallParentFunction)
  (if (Variables|Components|GetOnKeypad?)
    (Game|Player|SetViewTargetwithBlend (Game|GetPlayerController 0) (Components|GetOwner (.AsFirst%20Person%20Character (Utilities|Casting|CastToFirstPersonCharacter (Game|Player|GetPlayerPawn 0)))) 0.5 "VTBlend_Linear" 0.0 false)
    (bind _output_get (Variables|/Script/Engine.PlayerController|SetbShowMouseCursor _returnvalue_2 false))
    (bind _output_get_2 (Variables|/Script/Engine.PlayerController|SetbEnableClickEvents _returnvalue_2 _output_get))
    (Variables|/Script/Engine.PlayerController|SetbEnableMouseOverEvents _returnvalue_2 _output_get_2)
    (else
      (Variables|Components|SetOnKeypad? true)
      (Game|Player|SetViewTargetwithBlend (Game|GetPlayerController 0) (Components|GetOwner (Variables|Default|GetCamera)) 0.5 "VTBlend_Linear" 0.0 false)
      (bind _output_get_3 (Variables|/Script/Engine.PlayerController|SetbShowMouseCursor _returnvalue true))
      (bind _output_get_4 (Variables|/Script/Engine.PlayerController|SetbEnableClickEvents _returnvalue _output_get_3))
      (Variables|/Script/Engine.PlayerController|SetbEnableMouseOverEvents _returnvalue _output_get_4)
      (Rendering|Components|TextRender|SetText _code (Utilities|Text|MakeLiteralText (Utilities|Text|ToText(String) (Utilities|String|GetSubstring (Utilities|String|MakeLiteralString ".........") 0 (Utilities|String|Len (Variables|Components|GetKeypadCode))))))
      (Rendering|Components|TextRender|SetTextRenderColor _code (Math|Color|MakeColor 20 20 20 255))
      (bind _output_get_5 (Variables|Components|SetButtonsArray (Utilities|Array|MakeArray (Variables|Default|GetButtonNB0) (Variables|Default|GetButtonNB1) (Variables|Default|GetButtonNB2) (Variables|Default|GetButtonNB3) (Variables|Default|GetButtonNB4) (Variables|Default|GetButtonNB5) (Variables|Default|GetButtonNB6) (Variables|Default|GetButtonNB7) (Variables|Default|GetButtonNB8) (Variables|Default|GetButtonNB9) (Variables|Default|GetButtonOK) (Variables|Default|GetButtonNO))))
      (for _array_element _output_get_5
        (bind _asbutton_nb (Utilities|Casting|CastToButtonNB (Variables|/Script/Engine.ChildActorComponent|GetChildActor _array_element)))
        (Variables|/Game/AddedAssets/ButtonNB.ButtonNB_C|SetKeypadActorRef _asbutton_nb self)))))

(fn ConstructionScript
  (|CallParentFunction))