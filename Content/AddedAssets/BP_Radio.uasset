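; BP_Radio is an interactable radio prop that plays its AudioSHREK track from the start as soon as play begins.
; Its interaction event runs the parent Interact logic, then branches on Switch to stop the audio or restart it from the beginning.
; Switch is never set in this Blueprint, and the overlap and Tick events are empty.
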(event Custom|CustomEvent
  (|CallParentFunction)
  (switch int (Variables|Default|GetSwitch)
    (:0
      (Audio|Components|Audio|Stop (Variables|Default|GetAudio%20-%20SHREK)))
    (:1
      (Audio|Components|Audio|Play (Variables|Default|GetAudio%20-%20SHREK) 0.0))))

(event EventBeginPlay
  (|CallParentFunction)
  (Audio|Components|Audio|Play (Variables|Default|GetAudio%20-%20SHREK) 0.0))

(event Collision|EventActorBeginOverlap
  (params (OtherActor :type Actor%20Object%20Reference)))

(event EventTick
  (params (DeltaSeconds :type Float%20%28single-precision%29)))

(fn ConstructionScript
  (|CallParentFunction))