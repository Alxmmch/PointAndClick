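; BP_Lampe is a lamp that switches its point light on and off when interacted with.
; It overrides the parent's Interact event, flipping an IsOn flag and setting the PointLight intensity to full or zero rather than toggling visibility.
; BeginPlay marks the lamp as on without touching the light, so the initial brightness comes from the component's own settings.
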(event EventBeginPlay
  (|CallParentFunction)
  (Variables|Default|SetIsOn true))

(event Collision|EventActorBeginOverlap
  (params (OtherActor :type Actor%20Object%20Reference)))

(event EventTick
  (params (DeltaSeconds :type Float%20%28single-precision%29)))

(event EventInteract
  (|CallParentFunction)
  (bind _output_get (Variables|Default|SetIsOn (not (Variables|Default|GetIsOn))))
  (if _output_get
    (Rendering|Components|Light|SetIntensity (Variables|Default|GetPointLight) 5e+03)
    (else
      (Rendering|Components|Light|SetIntensity (Variables|Default|GetPointLight) 0.0))))

(fn ConstructionScript
  (|CallParentFunction))